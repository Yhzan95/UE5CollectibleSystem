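; BP_Collectible is a pickup the third-person character collects by overlap, with progress recorded per level, ID and type in the current save.
; On BeginPlay it registers its ID with BP_GI_Game, destroying itself if the ID is unset, registration returns true, or the save marks it collected.
; Overlap disables collision, writes to the save, notifies the game instance of new pickups with type, name and icon, then destroys the actor.
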(event `self.ReceiveBeginPlay`
  ;[0.003091 0.15 0 0.5] Initialize Collectible & Restore Saved State
  (if (== (`self.CollectibleID`) "None")
    (`self.K2_DestroyActor`)
    (else
      (bind _asbp_gi_game (cast `/Game/Collectible/Blueprints/BP_GI_Game` (`GameplayStatics.GetGameInstance`)))
      (bind _isduplicate (`/Game/Collectible/Blueprints/BP_GI_Game.RegisterCollectibleID` _asbp_gi_game (`self.CollectibleID`)))
      (if _isduplicate
        (`self.K2_DestroyActor`)
        (else
          (bind _currentsave (`/Game/Collectible/Blueprints/BP_GI_Game.CurrentSave` _asbp_gi_game))
          (`/Engine/EditorBlueprintResources/StandardMacros.IsValid` _currentsave
            (:`Is Valid`
              (bind _iscollected (`/Game/Collectible/Blueprints/SG_SaveGame.IsCollectibleCollected` _currentsave (`self.LevelID`) (`self.CollectibleID`) (`self.CollectibleType`)))
              (if _iscollected
                (`self.K2_DestroyActor`)))))))))

(event `self.InteractionCollision.OnComponentBeginOverlap`
  (params (OverlappedComponent :type "PrimitiveComponent Object Reference") (OtherActor :type "Actor Object Reference") (OtherComp :type "PrimitiveComponent Object Reference") (OtherBodyIndex :type Integer) (bFromSweep :type Boolean) (SweepResult :type "HitResult Structure (by ref)"))
  (bind _levelid (`self.LevelID`))
  ;[0.004637 0.15 0.000249 0.5] Handle Collectible Pickup & Update Progress
  (cast `/Game/ThirdPerson/Blueprints/BP_ThirdPersonCharacter` OtherActor)
  (if (not (`self.IsCollected`))
    (set `self.IsCollected` true)
    (`PrimitiveComponent.SetCollisionEnabled` (`self.InteractionCollision`) "NoCollision")
    (bind _asbp_gi_game (cast `/Game/Collectible/Blueprints/BP_GI_Game` (`GameplayStatics.GetGameInstance`)))
    (bind _currentsave (`/Game/Collectible/Blueprints/BP_GI_Game.CurrentSave` _asbp_gi_game))
    (`/Engine/EditorBlueprintResources/StandardMacros.IsValid` _currentsave
      (:`Is Valid`
        (bind _wasnewcollectible (`/Game/Collectible/Blueprints/SG_SaveGame.CollectCollectible` _currentsave _levelid (`self.CollectibleID`) (`self.CollectibleType`)))
        (if _wasnewcollectible
          (`/Game/Collectible/Blueprints/BP_GI_Game.OnCollectibleChanged` _asbp_gi_game)
          (`/Game/Collectible/Blueprints/BP_GI_Game.OnCollectiblePickedUp` _asbp_gi_game (`self.CollectibleType`) (`self.DisplayName`) (`self.Icon`))
          (`/Game/Collectible/Blueprints/SG_SaveGame.GetCollectibleCount` _currentsave _levelid "NewEnumerator0")
          (`/Game/Collectible/Blueprints/SG_SaveGame.GetCollectibleCount` _currentsave _levelid "NewEnumerator1")
          (`/Game/Collectible/Blueprints/SG_SaveGame.GetLevelCollectedCount` _currentsave _levelid)
          (switch `/Game/Collectible/Enumeration/E_CollectibleType` (`self.CollectibleType`)
            (:`NewEnumerator0`
              (`self.K2_DestroyActor`))
            (:`NewEnumerator1`
              (`self.K2_DestroyActor`)))
          (else
            (`self.K2_DestroyActor`)))))))

(fn `UserConstructionScript`)