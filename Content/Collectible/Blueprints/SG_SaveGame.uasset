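; SaveGame object that records which collectibles the player has picked up in each level, for two collectible types.
; A LevelProgress map keys each level ID to a struct holding one ID array per type.
; CollectCollectible rejects already collected IDs, otherwise adds the ID and writes the struct back through CommitLevelProgress, returning whether it was new.
; Query functions report collected state, per-type counts and the level total.
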(fn `CollectCollectible`
  (params (LevelID :type Name) (CollectibleID :type Name) (CollectibleType :type "/Game/Collectible/Enumeration/E_CollectibleType Enum" :default "NewEnumerator0"))
  (returns (WasNewCollectible :type Boolean))
  (locals (WorkingCollectible1IDs :type "Array of Name") (WorkingCollectible2IDs :type "Array of Name"))
  (bind _collectibleid (`local.CollectibleID`))
  (bind _levelid (`local.LevelID`))
  (bind _workingcollectible1ids (`local.WorkingCollectible1IDs`))
  (bind _workingcollectible2ids (`local.WorkingCollectible2IDs`))
  ; Register New Collectible & Update Level Progress
  (bind _iscollected (`self.IsCollectibleCollected` LevelID CollectibleID CollectibleType))
  (if _iscollected
    (return false)
    (else
      (bind _levelprogressresult (`self.GetLevelProgress` (`local.LevelID`)))
      (set `local.WorkingCollectible1IDs` (break `/Game/Collectible/Structs/ST_LevelProgress` _levelprogressresult))
      (set `local.WorkingCollectible2IDs` (`.CollectedCollectible2IDs_14_728C876043CC74B47C4CCDBD5D2D6813` (break `/Game/Collectible/Structs/ST_LevelProgress` _levelprogressresult)))
      (switch `/Game/Collectible/Enumeration/E_CollectibleType` (`local.CollectibleType`)
        (:`NewEnumerator0`
          (`KismetArrayLibrary.Array_AddUnique` (`local.WorkingCollectible1IDs`) _collectibleid)
          (`self.CommitLevelProgress` _levelid _workingcollectible1ids _workingcollectible2ids)
          (return true))
        (:`NewEnumerator1`
          (`KismetArrayLibrary.Array_AddUnique` (`local.WorkingCollectible2IDs`) _collectibleid)
          (`self.CommitLevelProgress` _levelid _workingcollectible1ids _workingcollectible2ids)
          (return true))))))

(fn `CommitLevelProgress`
  (params (LevelID :type Name) (Collectible1IDs :type "Array of Name") (Collectible2IDs :type "Array of Name"))
  ; Commit Level Collectible Progress
  (`BlueprintMapLibrary.Map_Add` (`self.LevelProgress`) LevelID (make `/Game/Collectible/Structs/ST_LevelProgress` Collectible1IDs Collectible2IDs)))

(fn `GetCollectibleCount`
  (params (LevelID :type Name) (CollectibleType :type "/Game/Collectible/Enumeration/E_CollectibleType Enum" :default "NewEnumerator0"))
  (returns (CollectedCount :type Integer))
  ; Get Collected Count by Type
  (bind (_levelprogressresult _found) (`self.GetLevelProgress` LevelID))
  (if _found
    (switch `/Game/Collectible/Enumeration/E_CollectibleType` (`local.CollectibleType`)
      (:`NewEnumerator0`
        (return (`KismetArrayLibrary.Array_Length` (break `/Game/Collectible/Structs/ST_LevelProgress` _levelprogressresult))))
      (:`NewEnumerator1`
        (return (`KismetArrayLibrary.Array_Length` (`.CollectedCollectible2IDs_14_728C876043CC74B47C4CCDBD5D2D6813` (break `/Game/Collectible/Structs/ST_LevelProgress` _levelprogressresult))))))
    (else
      (return 0))))

(fn `GetLevelCollectedCount`
  (params (LevelID :type Name))
  (returns (CollectedCount :type Integer))
  ; Get Total Collected Count for Level
  (bind _collectedcount (`self.GetCollectibleCount` LevelID))
  (bind _collectedcount_2 (`self.GetCollectibleCount` LevelID "NewEnumerator1"))
  (return (+ _collectedcount _collectedcount_2)))

(fn `GetLevelProgress`
  (params (LevelID :type Name))
  (returns (LevelProgressResult :type "/Game/Collectible/Structs/ST_LevelProgress Structure") (Found :type Boolean))
  (bind (_value _returnvalue) (`BlueprintMapLibrary.Map_Find` (`self.LevelProgress`) LevelID))
  ; Get Saved Level Progress
  (return _value _returnvalue))

(fn `IsCollectibleCollected`
  (params (LevelID :type Name) (CollectibleID :type Name) (CollectibleType :type "/Game/Collectible/Enumeration/E_CollectibleType Enum" :default "NewEnumerator0"))
  (returns (IsCollected :type Boolean))
  (bind _collectibleid (`local.CollectibleID`))
  ; Check If Collectible Is Already Collected
  (bind (_levelprogressresult _found) (`self.GetLevelProgress` LevelID))
  (if _found
    (switch `/Game/Collectible/Enumeration/E_CollectibleType` (`local.CollectibleType`)
      (:`NewEnumerator0`
        (return (`KismetArrayLibrary.Array_Contains` (break `/Game/Collectible/Structs/ST_LevelProgress` _levelprogressresult) _collectibleid)))
      (:`NewEnumerator1`
        (return (`KismetArrayLibrary.Array_Contains` (`.CollectedCollectible2IDs_14_728C876043CC74B47C4CCDBD5D2D6813` (break `/Game/Collectible/Structs/ST_LevelProgress` _levelprogressresult)) _collectibleid))))
    (else
      (return false))))